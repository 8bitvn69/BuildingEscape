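; BP_OpenableDoor is a door actor that swings open and closed.
; It stores its starting rotation on BeginPlay, and the OpenDoor component's OnOpen and OnClose events play or reverse the DoorSwing timeline.
; The timeline adds its yaw curve to the stored rotation each update, and a Play Sound event track plays the Doorlock sound at the door's location.
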(event OnOpen(OpenDoor)
  (bind _open_door (Timeline|Door%20Swing Play)
    (:Update
      (Transformation|SetActorRotation (Math|Rotator|CombineRotators (Math|Rotator|MakeRotator 0.0 0.0 _open_door) (Variables|Default|GetStart%20Rotation))))
    (:Play%20Sound
      (Audio|PlaySoundatLocation "/Game/SFX/door-lock.door-lock" (Transformation|GetActorLocation)))))

(event OnClose(OpenDoor)
  (bind _open_door (Timeline|Door%20Swing Reverse)
    (:Update
      (Transformation|SetActorRotation (Math|Rotator|CombineRotators (Math|Rotator|MakeRotator 0.0 0.0 _open_door) (Variables|Default|GetStart%20Rotation))))
    (:Play%20Sound
      (Audio|PlaySoundatLocation "/Game/SFX/door-lock.door-lock" (Transformation|GetActorLocation)))))

(event EventBeginPlay
  (Variables|Default|SetStart%20Rotation (Transformation|GetActorRotation)))

(fn ConstructionScript)